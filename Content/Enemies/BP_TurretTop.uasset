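; BP_TurretTop is the top part of an enemy turret that turns to face the player when it sees them.
; A PawnSensing component reports seen pawns, and for a CH_player the actor sets its rotation straight along the direction to that player's location.
; On its death event it notifies its spawner reference, if valid, that a monster died, then destroys itself.
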(event `self.PawnSensing.OnSeePawn`
  (params (Pawn :type "Pawn Object Reference"))
  (bind _asch_player (cast `/Game/Player/CH_player` Pawn))
  (`self.K2_SetActorRotation` self (`KismetMathLibrary.Conv_VectorToRotator` (- (`self.K2_GetActorLocation` _asch_player) (`self.K2_GetActorLocation` self))) false))

(event `Event_Death`
  (bind _ref_spawner (`self.ref_spawner`))
  (`/Engine/EditorBlueprintResources/StandardMacros.IsValid` _ref_spawner
    (:`Is Valid`
      (`/Game/WorldObjects/Triggerables/Triggers/BP_TSpawner.Event_NewMonsterDead` _ref_spawner))
    (:`Is Not Valid`
      _))
  (`self.K2_DestroyActor`))

(fn `UserConstructionScript`)