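; Blue half of a portal pair that teleports CH_player to the first BP_redPortal found in the level.
; Box overlap moves the player just in front of the red portal's Arrow, matches control yaw to it and calls StopMovement on the controller.
; Both portals' CanTeleport flags lock for a second to prevent bouncing back.
; With no red portal present, the blue portal stays disabled after the first player overlap.
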(event `self.Box.OnComponentBeginOverlap`
  (params (OverlappedComponent :type "PrimitiveComponent Object Reference") (OtherActor :type "Actor Object Reference") (OtherComp :type "PrimitiveComponent Object Reference") (OtherBodyIndex :type Integer) (bFromSweep :type Boolean) (SweepResult :type "HitResult Structure (by ref)"))
  (bind _returnvalue (`GameplayStatics.GetPlayerController` 0))
  (if (`self.canTeleport`)
    (bind _asch_player (cast `/Game/Player/CH_player` OtherActor))
    (set `self.canTeleport` false)
    (bind _outactors (`GameplayStatics.GetAllActorsOfClass` "/Game/Player/portals/BP_redPortal.BP_redPortal_C"))
    (if (> (`KismetArrayLibrary.Array_Length` _outactors) 0)
      (bind _output (`|GetArrayItem` _outactors))
      (set `/Game/Player/portals/BP_redPortal.canTeleport` false _output)
      (bind _returnvalue_2 (`SceneComponent.GetForwardVector` (`/Game/Player/portals/BP_redPortal.Arrow` _output)))
      (bind (_returnvalue_roll _returnvalue_pitch _returnvalue_yaw) (`KismetMathLibrary.BreakRotator` (`KismetMathLibrary.Conv_VectorToRotator` _returnvalue_2)))
      (`Controller.SetControlRotation` _returnvalue (`KismetMathLibrary.MakeRotator` 0.0 0.0 _returnvalue_yaw))
      (`self.K2_SetActorLocation` _asch_player (+ (`self.K2_GetActorLocation` _output) (* _returnvalue_2 70)) false true)
      (`Controller.StopMovement` _returnvalue)
      (`KismetSystemLibrary.Delay` 1.0)
      (set `self.canTeleport` true)
      (set `/Game/Player/portals/BP_redPortal.canTeleport` true _output))))

(fn `UserConstructionScript`)