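; Chak'Ak boss character, built from child-actor body parts linked into a map and a parent-child hierarchy.
; Destroyed-part checks drive three phases and death; later phases clear portals and send it to the nearest repair zone to reactivate parts with that phase's stats.
; Phase two also snaps the shoulder railguns into mirrored firing positions.
; It includes an enrage reactivation timer, queued audio, and add spawning that nothing here triggers.
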(event `self.ReceiveBeginPlay`
  ;[1 1 1] Begin Play
  (`parent.ReceiveBeginPlay`)
  (bind _asaic_chak_ak (cast `/Game/GameActors/Characters/AI/Boss/AIC_ChakAk` (`AIBlueprintHelperLibrary.GetAIController` self)))
  (set `self.AIC_chakak_ref` _asaic_chak_ak)
  (`self.Event_INIT`))

(event `Event_ChakAkDeath`
  (`KismetSystemLibrary.PrintString` "DEAD")
  (bind _values (`BlueprintMapLibrary.Map_Values` (`self.parts`)))
  (bind (_arrayindex _arrayelement) (`/Engine/EditorBlueprintResources/StandardMacros.ReverseForEachLoop` _values)
    (:`LoopBody`
      (`/Engine/EditorBlueprintResources/StandardMacros.IsValid` _arrayelement
        (:`Is Valid`
          (`self.K2_DestroyActor` _arrayelement))))))

(event `Event_ComponentDestroyed`
  (params (component :type "/Game/GameActors/Characters/AI/Utilities/enum_boss_parts Enum" :default "NewEnumerator0"))
  (bind _destroyedparts (`self.destroyedParts`))
  (`BlueprintMapLibrary.Map_Remove` _destroyedparts component)
  (`BlueprintMapLibrary.Map_Add` _destroyedparts component true)
  (`KismetSystemLibrary.PrintString` (`KismetStringLibrary.Concat_StrStr` (`|GetEnumeratorNameAsString` component) " Destroyed"))
  (`self.Event_CheckChangePhase`)
  (if (`|EnumEquality` component "NewEnumerator1")
    (`/Game/GameActors/Characters/AI/Boss/Components/Sub-Component/BPA_BC_head.Event_SetCoreState` (`self.head`) true)))

(event `Event_SetDestroyedMapToZeros`
  (bind _keys (`BlueprintMapLibrary.Map_Keys` (`self.parts`)))
  (for _array_element _keys
    (`BlueprintMapLibrary.Map_Add` (`self.destroyedParts`) _array_element)))

(event `Event_SetupChakAkVarComponents`
  (bind _asbpa_bc_head (cast `/Game/GameActors/Characters/AI/Boss/Components/Sub-Component/BPA_BC_head` (`ChildActorComponent.ChildActor` (`self.BPA_BC_head`))))
  (set `self.head` _asbpa_bc_head)
  (bind _asbpa_bc_core (cast `/Game/GameActors/Characters/AI/Boss/Components/Sub-Component/BPA_BC_core` (`ChildActorComponent.ChildActor` (`self.BPA_BC_core`))))
  (set `self.core` _asbpa_bc_core)
  (bind _asbpa_bc_arm (cast `/Game/GameActors/Characters/AI/Boss/Components/Sub-Component/BPA_BC_arm` (`ChildActorComponent.ChildActor` (`self.BPA_BC_arm_R`))))
  (set `self.arm_R` _asbpa_bc_arm)
  (bind _asbpa_bc_arm_2 (cast `/Game/GameActors/Characters/AI/Boss/Components/Sub-Component/BPA_BC_arm` (`ChildActorComponent.ChildActor` (`self.BPA_BC_arm_L`))))
  (set `self.arm_L` _asbpa_bc_arm_2)
  (bind _asbpa_bc_melee (cast `/Game/GameActors/Characters/AI/Boss/Components/Sub-Component/BPA_BC_melee` (`ChildActorComponent.ChildActor` (`self.BPA_BC_melee_R`))))
  (set `self.melee_R` _asbpa_bc_melee)
  (bind _asbpa_bc_melee_2 (cast `/Game/GameActors/Characters/AI/Boss/Components/Sub-Component/BPA_BC_melee` (`ChildActorComponent.ChildActor` (`self.BPA_BC_melee_L`))))
  (set `self.melee_L` _asbpa_bc_melee_2)
  (bind _asbpa_bc_shoulder (cast `/Game/GameActors/Characters/AI/Boss/Components/Sub-Component/BPA_BC_shoulder` (`ChildActorComponent.ChildActor` (`self.BPA_BC_shoulder_R`))))
  (set `self.shoulder_R` _asbpa_bc_shoulder)
  (bind _asbpa_bc_shoulder_2 (cast `/Game/GameActors/Characters/AI/Boss/Components/Sub-Component/BPA_BC_shoulder` (`ChildActorComponent.ChildActor` (`self.BPA_BC_shoulder_L`))))
  (set `self.shoulder_L` _asbpa_bc_shoulder_2)
  (`self.Event_FeedComponentArray`))

(event `Event_FeedComponentArray`
  (set `self.components` (`|MakeArray` (`self.head`) (`self.core`) (`self.shoulder_R`) (`self.shoulder_L`) (`self.arm_R`) (`self.arm_L`) (`self.melee_R`) (`self.melee_L`) :!type "/Game/GameActors/Characters/AI/Boss/Components/BPA_BossComponent Object Reference"))
  (`self.Event_FeedPartsMap`))

(event `Event_FeedPartsMap`
  (for _array_element (`self.components`)
    (`BlueprintMapLibrary.Map_Add` (`self.parts`) (`/Game/GameActors/Characters/AI/Boss/Components/BPA_BossComponent.partType` _array_element) _array_element))
  (`self.Event_SetChakAkRefInAllComponents`))

(event `Event_SetChildComponents`
  (bind _melee_l (`self.melee_L`))
  (bind _arm_l (`self.arm_L`))
  (bind _melee_r (`self.melee_R`))
  (bind _shoulder_r (`self.shoulder_R`))
  (bind _core (`self.core`))
  (bind _shoulder_l (`self.shoulder_L`))
  (bind _arm_r (`self.arm_R`))
  (`/Game/GameActors/Characters/AI/Boss/Components/BPA_BossComponent.Event_setChildPart` (`self.head`) (`/Game/GameActors/Characters/AI/Boss/Components/BPA_BossComponent.partType` _core) _core)
  (`/Game/GameActors/Characters/AI/Boss/Components/BPA_BossComponent.Event_setChildPart` (`self.core`) (`/Game/GameActors/Characters/AI/Boss/Components/BPA_BossComponent.partType` _arm_r) _arm_r)
  (`/Game/GameActors/Characters/AI/Boss/Components/BPA_BossComponent.Event_setChildPart` (`self.core`) (`/Game/GameActors/Characters/AI/Boss/Components/BPA_BossComponent.partType` _arm_l) _arm_l)
  (`/Game/GameActors/Characters/AI/Boss/Components/BPA_BossComponent.Event_setChildPart` (`self.core`) (`/Game/GameActors/Characters/AI/Boss/Components/BPA_BossComponent.partType` _shoulder_r) _shoulder_r)
  (`/Game/GameActors/Characters/AI/Boss/Components/BPA_BossComponent.Event_setChildPart` (`self.core`) (`/Game/GameActors/Characters/AI/Boss/Components/BPA_BossComponent.partType` _shoulder_l) _shoulder_l)
  (`/Game/GameActors/Characters/AI/Boss/Components/BPA_BossComponent.Event_setChildPart` (`self.arm_R`) (`/Game/GameActors/Characters/AI/Boss/Components/BPA_BossComponent.partType` _melee_r) _melee_r)
  (`/Game/GameActors/Characters/AI/Boss/Components/BPA_BossComponent.Event_setChildPart` (`self.arm_L`) (`/Game/GameActors/Characters/AI/Boss/Components/BPA_BossComponent.partType` _melee_l) _melee_l)
  (`self.Event_InitFinished`))

(event `Event_INIT`
  (`self.Event_SetupChakAkVarComponents`))

(event `Event_SetChakAkRefInAllComponents`
  (for _array_element (`self.components`)
    (`/Game/GameActors/Characters/AI/Boss/Components/BPA_BossComponent.Event_SetBossRef` _array_element self))
  (`self.Event_SetChildComponents`))

(event `Event Destroy Portals`
  (bind _outactors (`GameplayStatics.GetAllActorsOfClass` "/Game/GameActors/WorldObjects/InteractibleObjects/Interactibles/Portals/Int_Portal.Int_Portal_C"))
  (for _array_element _outactors
    (`/Engine/EditorBlueprintResources/StandardMacros.IsValid` _array_element
      (:`Is Valid`
        (`self.K2_DestroyActor` _array_element)))))

(event `Event Slow Player`)

(event `Event Gravity Change`)

(event `Event_CheckChangePhase`
  (if (`self.phase_2`)
    (`self.Event_SetPhase` "NewEnumerator1")
    (`self.Event_RailgunsInPosition`)
    (elif (`self.phase_3`)
      (`self.Event_SetPhase` "NewEnumerator3")
      (elif (`self.death`)
        (`self.Event_ChakAkDeath`)))))

(event `Event_SetActivateComponents`
  (bind (_max_hp _armour) (break `/Game/GameActors/Characters/AI/Utilities/struct_bossStats` (`BlueprintMapLibrary.Map_Find` (`self.phaseStats`) (`self.phase`))))
  (`KismetSystemLibrary.Delay` 0.2)
  (bind (_arrayindex _arrayelement) (`/Engine/EditorBlueprintResources/StandardMacros.ReverseForEachLoop` (`self.components`))
    (:`LoopBody`
      (`/Game/GameActors/Characters/AI/Boss/Components/BPA_BossComponent.Event_ActivateComponent` _arrayelement _max_hp _armour))))

(event `Event_InitFinished`
  (`self.Event_SetPhase` "NewEnumerator0"))

(event `Event_SetPhase`
  (params (phase :type "/Game/GameActors/Characters/AI/Utilities/enum_phases Enum" :default "NewEnumerator0"))
  (bind _output_get (set `self.phase` phase))
  (`KismetSystemLibrary.PrintString` (`KismetStringLibrary.Concat_StrStr` "New Phase : " (`|GetEnumeratorNameAsString` _output_get)) true true (struct :`R` 1.0 :`G` 0.065432 :`A` 1.0) 10.0)
  (`self.Event_SetDestroyedMapToZeros`)
  (`self.Event Destroy Portals`)
  (`/Game/GameActors/Characters/AI/Boss/Components/Sub-Component/BPA_BC_head.Event_SetCoreState` (`self.head`) false)
  (if (`|EnumInequality` (`self.phase`) "NewEnumerator0")
    (`self.Event_MoveToRepairZone`)))

(event `Event_EnragedToggle`
  (params (isEnraged :type Boolean))
  (bind _output_get (set `self.isEnraged` isEnraged))
  (`KismetSystemLibrary.K2_SetTimerDelegate` (delegate `Event_EnragedMode`) (`self.respawnDelay`) _output_get))

(event `Event_EnragedMode`
  (`self.Event_FindComponentToSpawn`))

(event `Event_PlaySound`
  (params (sound :type "/Game/GameActors/Characters/AI/Utilities/enum_sound Enum" :default "NewEnumerator0"))
  (`KismetArrayLibrary.Array_Add` (`self.soundQueue`) (`BlueprintMapLibrary.Map_Find` (`self.soundPlaylist`) sound))
  (`self.Event_Playlist`))

(event `Event_Playlist`
  (bind _audiocurvesource (`self.AudioCurveSource`))
  (bind _soundqueue (`self.soundQueue`))
  (if (not (`AudioComponent.IsPlaying` (`self.AudioCurveSource`)))
    (bind (_arrayindex _arrayelement) (`/Engine/EditorBlueprintResources/StandardMacros.ReverseForEachLoop` _soundqueue)
      (:`LoopBody`
        (`/Engine/EditorBlueprintResources/StandardMacros.IsValid` _arrayelement
          (:`Is Valid`
            (`KismetSystemLibrary.Delay` 2.0)
            (`AudioComponent.SetSound` _audiocurvesource _arrayelement)
            (`KismetArrayLibrary.Array_RemoveItem` _soundqueue _arrayelement)
            (`AudioComponent.SetVolumeMultiplier` _audiocurvesource 0.4)
            (`AudioComponent.Play` _audiocurvesource 0.0)))))))

(event `self.AudioCurveSource.OnAudioFinished`
  (`self.Event_Playlist`))

(event `Event_SpawnAdds`
  (for _array_element (`self.addsToSpawn`)
    (bind _outactors (`GameplayStatics.GetAllActorsOfClass` "/Game/GameActors/Characters/AI/Utilities/BPA_BossAddsSpawner.BPA_BossAddsSpawner_C"))
    (bind _actor (`/Game/Libs/Library.randomElementOfArray` _outactors))
    (`/Engine/EditorBlueprintResources/StandardMacros.IsValid` _actor
      (:`Is Valid`
        (bind (_aiclass _number) (break `/Game/GameActors/Characters/AI/Utilities/struct_bossAdds` _array_element))
        (for _ (range (+ _number 1))
          (`AIBlueprintHelperLibrary.SpawnAIFromClass` _aiclass null (`self.K2_GetActorLocation` _actor)))))))

(event `Event_setAddsToSpawn`
  (`KismetArrayLibrary.Array_Clear` (`self.addsToSpawn`))
  (switch `/Game/GameActors/Characters/AI/Utilities/enum_phases` (`self.phase`)
    (:`NewEnumerator0`
      (set `self.addsToSpawn` (`|MakeArray` (make `/Game/GameActors/Characters/AI/Utilities/struct_bossAdds` "/Game/AIC_Zombie.AIC_Zombie_C" 5))))
    (:`NewEnumerator1`
      (set `self.addsToSpawn` (`|MakeArray` (make `/Game/GameActors/Characters/AI/Utilities/struct_bossAdds` "/Game/AIC_Zombie.AIC_Zombie_C" 7) (make `/Game/GameActors/Characters/AI/Utilities/struct_bossAdds` "/Game/GameActors/Characters/AI/Ranger/AIC_Ranger.AIC_Ranger_C" 5))))
    (:`NewEnumerator3`
      (set `self.addsToSpawn` (`|MakeArray` (make `/Game/GameActors/Characters/AI/Utilities/struct_bossAdds` "/Game/AIC_Zombie.AIC_Zombie_C" 10) (make `/Game/GameActors/Characters/AI/Utilities/struct_bossAdds` "/Game/GameActors/Characters/AI/Ranger/AIC_Ranger.AIC_Ranger_C" 7) (make `/Game/GameActors/Characters/AI/Utilities/struct_bossAdds` "/Game/GameActors/Characters/AI/Ranger/AIC_Ranger.AIC_Ranger_C" 5)))))
  (`self.Event_SpawnAdds`))

(event `Event_MoveToRepairZone`
  (bind _outactors (`GameplayStatics.GetAllActorsOfClass` "/Game/GameActors/Characters/AI/Utilities/BPA_BossRepairZone.BPA_BossRepairZone_C"))
  (bind _location (`/Game/Libs/Library.closestElementOfArrayFromTarget` _outactors self))
  (`|AIMoveTo` self _location null
    (:`OnSuccess`
      (`self.Event_SetActivateComponents`))))

(event `Event_FindComponentToSpawn`
  (bind _destroyedparts (`self.destroyedParts`))
  (bind (_max_hp _armour) (break `/Game/GameActors/Characters/AI/Utilities/struct_bossStats` (`BlueprintMapLibrary.Map_Find` (`self.phaseStats`) (`self.phase`))))
  (bind _keys (`BlueprintMapLibrary.Map_Keys` _destroyedparts))
  (for _array_element _keys
    (if (not (`BlueprintMapLibrary.Map_Find` _destroyedparts _array_element))
      (bind _value (`BlueprintMapLibrary.Map_Find` (`self.parts`) _array_element))
      (`/Engine/EditorBlueprintResources/StandardMacros.IsValid` _value
        (:`Is Valid`
          (`/Game/GameActors/Characters/AI/Boss/Components/BPA_BossComponent.Event_ActivateComponent` _value _max_hp _armour))))))

(event `Event_RailgunsInPosition`
  (bind _fireposition (`self.firePosition`))
  (`self.K2_SetActorRelativeTransform` (`self.shoulder_R`) _fireposition false true)
  (`self.K2_SetActorRelativeTransform` (`self.shoulder_L`) (`self.setYLocationToNegative` _fireposition) false true))

(event `self.ReceiveActorBeginOverlap`
  (params (OtherActor :type "Actor Object Reference"))
  (`parent.ReceiveActorBeginOverlap` OtherActor))

(fn `setYLocationToNegative`
  (params (InTransform :type "Transform Structure (by ref)"))
  (returns (ReturnValue :type "Transform Structure"))
  (return (`KismetMathLibrary.MakeTransform` (`KismetMathLibrary.MakeVector` (.x (.location InTransform)) (* (.y (.location InTransform)) -1.0) (.z (.location InTransform))) (.rotation InTransform) (.scale InTransform))))

(fn `UserConstructionScript`
  (`parent.UserConstructionScript`))