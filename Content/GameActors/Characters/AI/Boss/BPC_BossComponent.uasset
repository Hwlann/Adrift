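; Destructible body part of the ChakAk boss, with its own HP, armour, part type and map of child parts.
; Construction pulls base armour and max HP from the boss via its AI controller, and an armour event adds child parts' armour.
; Damage multiplies HP by an armour-adjusted amount.
; At zero HP it destroys its children and itself, triggering boss death for the Head or enrage for the Core.
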(event `self.TakeDamages`
  (params (amount :type Integer))
  ;[1 1 1] Damages & Death
  (set `self.hp` (`KismetMathLibrary.FTrunc` (* (`self.hp`) (* amount (`/Game/Libs/Library.dmgOutputWithArmor` (`self.armour`))))))
  (`self.Event_CheckDeath`))

(event `Event_CheckDeath`
  (bind _chakak (`self.ChakAk`))
  ;[1 1 1] Damages & Death
  (if (not (> (`self.hp`) 0))
    (`self.Event_DestroyChildElement`)
    (`self.K2_DestroyActor`)
    (switch `/Game/GameActors/Characters/AI/Utilities/enum_boss_parts` (`self.partType`)
      (:`NewEnumerator0`
        (`/Game/GameActors/Characters/AI/Boss/BPC_Chak_ak.Event_ChakAkDeath` _chakak))
      (:`NewEnumerator1`
        (`/Game/GameActors/Characters/AI/Boss/BPC_Chak_ak.Event_Enraged` _chakak)))))

(event `Event_DestroyChildElement`
  ;[1 1 1] Damages & Death
  (bind _values (`BlueprintMapLibrary.Map_Values` (`self.childPart`)))
  (for _array_element _values
    (`/Engine/EditorBlueprintResources/StandardMacros.IsValid` _array_element
      (:`Is Valid`
        (`self.K2_DestroyActor` _array_element)))))

(event `Event_FixArmor`
  ;[1 1 1] Armor
  (bind _values (`BlueprintMapLibrary.Map_Values` (`self.childPart`)))
  (for _array_element _values
    (`/Engine/EditorBlueprintResources/StandardMacros.IsValid` _array_element
      (:`Is Valid`
        (set `self.armour` (+ (`/Game/GameActors/Characters/AI/Boss/BPC_BossComponent.armour` _array_element) (`self.armour`)))))))

(fn `UserConstructionScript`
  (`parent.UserConstructionScript`)
  (bind _asaic_chak_ak (cast `/Game/GameActors/Characters/AI/Boss/AIC_ChakAk` (`AIBlueprintHelperLibrary.GetAIController` self)))
  (set `self.AIC_chakAk` _asaic_chak_ak)
  (bind _output_get (set `self.ChakAk` (`/Game/GameActors/Characters/AI/Boss/AIC_ChakAk.BP_chakak` _asaic_chak_ak)))
  (set `self.armour` (`/Game/GameActors/Characters/AI/Boss/BPC_Chak_ak.BaseArmour` _output_get))
  (set `self.hp` (`/Game/GameActors/Characters/AI/Char_AI.max_hp` _output_get)))