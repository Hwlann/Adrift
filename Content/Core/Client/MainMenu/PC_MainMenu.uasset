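; Main menu player controller that shows the menu widget, plays music and handles level loading, quitting, video switching and graphics settings.
; BeginPlay sets UI-only input and runs a timeline fading in menu and title opacity.
; Each timeline update also reapplies VSync and frame cap, then sets maximum scalability and resolution.
; Level opening looks up names in the menu GameMode's map by mode, falling back to that mode's first level.
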(event `self.ReceiveBeginPlay`
  (bind _w_mainmenucore (`self.W_mainMenuCore`))
  (bind _asgm_main_menu (cast `/Game/Core/Server/GM_MainMenu` (`GameplayStatics.GetGameMode`)))
  (set `self.GM_MainMenu` _asgm_main_menu)
  (bind _returnvalue (`|CreateWidget` "/Game/Widgets/MainMenu/W_MainMenuCore.W_MainMenuCore_C"))
  (bind _output_get (set `self.W_mainMenuCore` _returnvalue))
  (`Widget.SetRenderOpacity` (`/Game/Widgets/MainMenu/W_MainMenuCore.WS_Menu` _returnvalue) 0.0)
  (`WidgetBlueprintLibrary.SetInputMode_UIOnlyEx` self null)
  (`GameplayStatics.PlaySound2D` "/Game/Resources/Sounds/Music/Portal-SelfEsteemFund.Portal-SelfEsteemFund" 1.0 1.0 0.0 null null)
  (set `self.bShowMouseCursor` true)
  (`UserWidget.AddToViewport` _output_get 0)
  (bind (_direction _opacity _title_opacity) (`Timeline|Main_Widget`)
    (:`Update`
      (`Widget.SetRenderOpacity` (`/Game/Widgets/MainMenu/W_MainMenuCore.WS_Menu` _w_mainmenucore) _opacity)
      (`Widget.SetRenderOpacity` (`/Game/Widgets/MainMenu/W_MainMenuCore.txt_gameName` _w_mainmenucore) _title_opacity)
      (bind _returnvalue_2 (`GameUserSettings.GetGameUserSettings`))
      (`GameUserSettings.SetVSyncEnabled` _returnvalue_2 true)
      (`GameUserSettings.SetFrameRateLimit` _returnvalue_2 60.0)
      (`GameUserSettings.ApplySettings` _returnvalue_2 true)
      (`self.Event_changeGraphics` 4))))

(event `Event_OpenLevel`
  (params (LevelName :type Name))
  (bind (_value _returnvalue) (`BlueprintMapLibrary.Map_Find` (`/Game/Core/Server/GM_MainMenu.levelNames` (`self.GM_MainMenu`)) (`self.gameMode`)))
  (bind _returnvalue_2 (`KismetArrayLibrary.Array_Find` (break `/Game/Core/Server/Struct_NameArray` _value) LevelName))
  (if _returnvalue
    (if (`KismetArrayLibrary.Array_IsValidIndex` (break `/Game/Core/Server/Struct_NameArray` _value) _returnvalue_2)
      (set `self.bShowMouseCursor` false)
      (`GameplayStatics.OpenLevel` (`|GetArrayItem` (break `/Game/Core/Server/Struct_NameArray` _value) _returnvalue_2))
      (else
        (`GameplayStatics.OpenLevel` (`|GetArrayItem` (break `/Game/Core/Server/Struct_NameArray` _value)))))))

(event `Event_QuitGame`
  (`KismetSystemLibrary.QuitGame` null "Quit"))

(event `Event_ChangeMenuVideoSource`
  (params (indexOfVideoToPlay :type Integer))
  (bind _mp_mainmenuplayer (`self.MP_mainMenuPlayer`))
  (bind _output (`|GetArrayItem` (`|MakeArray` null null :!type "MediaSource Object Reference") indexOfVideoToPlay))
  (`/Engine/EditorBlueprintResources/StandardMacros.IsValid` _mp_mainmenuplayer
    (:`Is Valid`
      (`/Engine/EditorBlueprintResources/StandardMacros.IsValid` _output
        (:`Is Valid`
          (`MediaPlayer.OpenSource` _mp_mainmenuplayer _output))))))

(event `Event_changeGraphics`
  (params (level :type Integer))
  (bind _returnvalue (`KismetMathLibrary.Clamp` level 0 4))
  (bind _returnvalue_2 (`GameUserSettings.GetGameUserSettings`))
  (`GameUserSettings.SetAntiAliasingQuality` _returnvalue_2 _returnvalue)
  (`GameUserSettings.SetPostProcessingQuality` _returnvalue_2 _returnvalue)
  (`GameUserSettings.SetShadingQuality` _returnvalue_2 _returnvalue)
  (`GameUserSettings.SetShadowQuality` _returnvalue_2 _returnvalue)
  (`GameUserSettings.SetTextureQuality` _returnvalue_2 _returnvalue)
  (`GameUserSettings.SetViewDistanceQuality` _returnvalue_2 _returnvalue)
  (`GameUserSettings.SetVisualEffectQuality` _returnvalue_2 _returnvalue)
  (`GameUserSettings.SetScreenResolution` _returnvalue_2 (make `IntPoint` 1920 1080)))

(event `Event_ApplySetting`
  (bind _returnvalue (`GameUserSettings.GetGameUserSettings`))
  (`GameUserSettings.ApplySettings` _returnvalue true))

(fn `UserConstructionScript`)