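; Server game mode for speedrun play that reads a token from the command line and provides map rotation.
; On BeginPlay it splits command-line arguments on "=" and stores the right-hand value in BP_Instance's Token, without checking the key.
; Arguments without "=" print an invalid-token message.
; GetNextLevel finds the current level in the Maps array and returns the following entry, wrapping to the first at the end.
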(event `self.ReceiveBeginPlay`
  (bind _returnvalue (`KismetSystemLibrary.GetCommandLine`))
  (bind _asbp_instance (cast `/Game/_old/BP_Instance` (`GameplayStatics.GetGameInstance`)))
  (for _array_element (`KismetStringLibrary.ParseIntoArray` _returnvalue)
    (bind (_lefts _rights _returnvalue_2) (`KismetStringLibrary.Split` _array_element "="))
    (if _returnvalue_2
      (set `/Game/_old/BP_Instance.token` _rights _asbp_instance)
      (else
        (`KismetSystemLibrary.PrintString` (`KismetStringLibrary.Concat_StrStr` "UNVALID TOKEN" ":" _rights) true true (struct :`R` 1.0 :`G` 0.027671 :`A` 1.0) 10.0)))))

(fn `GetNextLevel`
  (returns (nextLevel :type Name))
  (bind _maps (`self.maps`))
  (bind _returnvalue (`GameplayStatics.GetCurrentLevelName` true))
  (bind _returnvalue_2 (+ (`KismetArrayLibrary.Array_Find` (`self.maps`) (`KismetStringLibrary.Conv_StringToName` _returnvalue)) 1))
  (if (`KismetArrayLibrary.Array_IsValidIndex` _maps _returnvalue_2)
    (return (`|GetArrayItem` _maps _returnvalue_2))
    (else
      (return (`|GetArrayItem` (`self.maps`))))))

(fn `UserConstructionScript`)