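; BP_Finish is a level finish trigger that ends the run when the player overlaps its Box.
; The overlap passes a DoOnce before the cast to CH_player, so any first overlapping actor consumes it.
; For a player, it disables input, shows W_VictoryScreen, then has player 0's pawn add ScoreValue, stop its timer and send the score.
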(event `self.Box.OnComponentBeginOverlap`
  (params (OverlappedComponent :type "PrimitiveComponent Object Reference") (OtherActor :type "Actor Object Reference") (OtherComp :type "PrimitiveComponent Object Reference") (OtherBodyIndex :type Integer) (bFromSweep :type Boolean) (SweepResult :type "HitResult Structure (by ref)"))
  (`/Engine/EditorBlueprintResources/StandardMacros.DoOnce` false
    (:`Completed`
      (bind _asch_player (cast `/Game/_old/Player/CH_player` OtherActor))
      (`self.DisableInput` _asch_player null)
      (bind _returnvalue (`|CreateWidget` "/Game/Widgets/Levels/W_VictoryScreen.W_VictoryScreen_C"))
      (`UserWidget.AddToViewport` _returnvalue 0)
      (bind _asch_player_2 (cast `/Game/_old/Player/CH_player` (`Controller.K2_GetPawn` (`GameplayStatics.GetPlayerController` 0))))
      (`/Game/_old/Player/CH_player.AddToScore` _asch_player_2 (`self.scoreValue`))
      (`/Game/_old/Player/CH_player.Event_StopTimer` _asch_player_2)
      (`/Game/_old/Player/CH_player.Event_SendScore` _asch_player_2))))

(fn `UserConstructionScript`)