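; BP_DashableArea is a trigger volume that lets the player dash while inside it.
; Box overlap events cast the other actor to CH_player, setting CanDash on entry and clearing it on exit.
; They also shift the camera FOV toward a wider value on entry and a narrower one on exit, using a single Lerp step per event, so the change is instant and partial.
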(event `self.Box.OnComponentBeginOverlap`
  (params (OverlappedComponent :type "PrimitiveComponent Object Reference") (OtherActor :type "Actor Object Reference") (OtherComp :type "PrimitiveComponent Object Reference") (OtherBodyIndex :type Integer) (bFromSweep :type Boolean) (SweepResult :type "HitResult Structure (by ref)"))
  (bind _asch_player (cast `/Game/_old/Player/CH_player` OtherActor))
  (bind _camera (`/Game/_old/Player/CH_player.Camera` _asch_player))
  (`CameraComponent.SetFieldOfView` _camera (`KismetMathLibrary.Lerp` (`CameraComponent.FieldOfView` _camera) 140.0 0.3))
  (set `/Game/_old/Player/CH_player.canDash` true _asch_player))

(event `self.Box.OnComponentEndOverlap`
  (params (OverlappedComponent :type "PrimitiveComponent Object Reference") (OtherActor :type "Actor Object Reference") (OtherComp :type "PrimitiveComponent Object Reference") (OtherBodyIndex :type Integer))
  (bind _asch_player (cast `/Game/_old/Player/CH_player` OtherActor))
  (bind _camera (`/Game/_old/Player/CH_player.Camera` _asch_player))
  (`CameraComponent.SetFieldOfView` _camera (`KismetMathLibrary.Lerp` (`CameraComponent.FieldOfView` _camera) 90.0 0.3))
  (set `/Game/_old/Player/CH_player.canDash` false _asch_player))

(fn `UserConstructionScript`)