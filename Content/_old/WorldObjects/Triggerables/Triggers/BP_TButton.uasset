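; One-shot interactable button that the player presses with E to award score and fire a linked trigger.
; The box overlap shows a prompt widget and unpauses a fast looping timer that polls for the key, pausing it again on exit.
; A press hides the prompt and plays a timeline offsetting the cylinder vertically.
; When the timeline finishes, it sets Activate, adds score to CH_player and calls Trigger on BpTrigger.
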(event `self.ReceiveBeginPlay`
  (bind _returnvalue (`KismetSystemLibrary.K2_SetTimerDelegate` (delegate `WaitPush`) 0.01 true))
  (bind _output_get (set `self.pushTimer` _returnvalue))
  (`KismetSystemLibrary.K2_PauseTimerHandle` _output_get))

(event `WaitPush`
  (if (and (`PlayerController.WasInputKeyJustPressed` (`GameplayStatics.GetPlayerController` 0) "E") (`self.isInRange`) (not (`self.activate`)))
    (`SceneComponent.SetHiddenInGame` (`self.Widget`) true true)
    (bind (_direction _newtrack_0) (`Timeline|Timeline_0` :!via `PlayFromStart`)
      (:`Update`
        (`SceneComponent.K2_AddWorldOffset` (`self.Cylinder`) (`KismetMathLibrary.MakeVector` 0.0 0.0 _newtrack_0) false false))
      (:`Finished`
        (set `self.activate` true)
        (bind _asch_player (cast `/Game/_old/Player/CH_player` (`Controller.K2_GetPawn` (`GameplayStatics.GetPlayerController` 0))))
        (`/Game/_old/Player/CH_player.AddToScore` _asch_player 100)
        (`/Game/_old/WorldObjects/Triggerables/BP_BlueprintTriggerable.Trigger` (`self.Bp_Trigger`))))))

(event `self.Box.OnComponentBeginOverlap`
  (params (OverlappedComponent :type "PrimitiveComponent Object Reference") (OtherActor :type "Actor Object Reference") (OtherComp :type "PrimitiveComponent Object Reference") (OtherBodyIndex :type Integer) (bFromSweep :type Boolean) (SweepResult :type "HitResult Structure (by ref)"))
  (cast `/Game/_old/Player/CH_player` OtherActor)
  (if (not (`self.activate`))
    (set `self.isInRange` true)
    (`SceneComponent.SetVisibility` (`self.Widget`) true false)
    (`KismetSystemLibrary.K2_UnPauseTimerHandle` (`self.pushTimer`))))

(event `self.Box.OnComponentEndOverlap`
  (params (OverlappedComponent :type "PrimitiveComponent Object Reference") (OtherActor :type "Actor Object Reference") (OtherComp :type "PrimitiveComponent Object Reference") (OtherBodyIndex :type Integer))
  (cast `/Game/_old/Player/CH_player` OtherActor)
  (set `self.isInRange` false)
  (`SceneComponent.SetVisibility` (`self.Widget`) false false)
  (`KismetSystemLibrary.K2_PauseTimerHandle` (`self.pushTimer`)))

(fn `UserConstructionScript`)