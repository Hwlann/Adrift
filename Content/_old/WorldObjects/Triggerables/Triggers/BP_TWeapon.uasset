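; Weapon pickup trigger that lets the player equip a weapon by pressing E nearby.
; Box overlap stores the player, shows a prompt widget and unpauses a looping timer that polls for the key instead of using Tick; leaving hides and pauses it.
; A one-time press hides the weapon and prompt, calls the player's equip event, awards score and fires BpTriggerable to trigger linked behavior.
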(event `self.ReceiveBeginPlay`
  (bind _returnvalue (`KismetSystemLibrary.K2_SetTimerDelegate` (delegate `WaitPush`) 0.01 true))
  (bind _output_get (set `self.pushTimer` _returnvalue))
  (`KismetSystemLibrary.K2_PauseTimerHandle` _output_get))

(event `WaitPush`
  (if (and (`PlayerController.WasInputKeyJustPressed` (`GameplayStatics.GetPlayerController` 0) "E") (`self.isInRange`) (not (`self.activate`)))
    (`/Engine/EditorBlueprintResources/StandardMacros.DoOnce` false
      (:`Completed`
        (set `self.activate` true)
        (`SceneComponent.SetHiddenInGame` (`self.weapon`) true true)
        (`SceneComponent.SetHiddenInGame` (`self.Widget`) true true)
        (`/Game/_old/Player/CH_player.Event_EquipWeapon` (`self.player`))
        (bind _asch_player (cast `/Game/_old/Player/CH_player` (`Controller.K2_GetPawn` (`GameplayStatics.GetPlayerController` 0))))
        (`/Game/_old/Player/CH_player.AddToScore` _asch_player 500)
        (`/Game/_old/WorldObjects/Triggerables/BP_BlueprintTriggerable.Trigger` (`self.bpTriggerable`))))))

(event `self.Box.OnComponentBeginOverlap`
  (params (OverlappedComponent :type "PrimitiveComponent Object Reference") (OtherActor :type "Actor Object Reference") (OtherComp :type "PrimitiveComponent Object Reference") (OtherBodyIndex :type Integer) (bFromSweep :type Boolean) (SweepResult :type "HitResult Structure (by ref)"))
  (if (not (`self.activate`))
    (bind _asch_player (cast `/Game/_old/Player/CH_player` OtherActor))
    (set `self.player` _asch_player)
    (set `self.isInRange` true)
    (`SceneComponent.SetVisibility` (`self.Widget`) true false)
    (`KismetSystemLibrary.K2_UnPauseTimerHandle` (`self.pushTimer`))))

(event `self.Box.OnComponentEndOverlap`
  (params (OverlappedComponent :type "PrimitiveComponent Object Reference") (OtherActor :type "Actor Object Reference") (OtherComp :type "PrimitiveComponent Object Reference") (OtherBodyIndex :type Integer))
  (set `self.isInRange` false)
  (`SceneComponent.SetVisibility` (`self.Widget`) false false)
  (`KismetSystemLibrary.K2_PauseTimerHandle` (`self.pushTimer`)))

(fn `UserConstructionScript`)