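; BP_Ammo is a portal-gun projectile that places a portal on portalable walls or kills zombies on hit.
; On a BP_PortalableWall it destroys existing portals of its type, then spawns one just off the surface, oriented along the hit normal.
; IsBlue picks the class, with true mapping to BP_redPortal and false to BP_bluePortal.
; Any other hit triggers death on a CH_Zombie, and the ammo destroys itself after every hit.
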(event `self.ReceiveHit`
  (params (MyComp :type "PrimitiveComponent Object Reference") (Other :type "Actor Object Reference") (OtherComp :type "PrimitiveComponent Object Reference") (bSelfMoved :type Boolean) (HitLocation :type "Vector Structure") (HitNormal :type "Vector Structure") (NormalImpulse :type "Vector Structure") (Hit :type "HitResult Structure (by ref)"))
  (bind _returnvalue (select `bool` (`self.isBlue`) :`false` "/Game/_old/Player/portals/BP_bluePortal.BP_bluePortal_C" :`true` "/Game/_old/Player/portals/BP_redPortal.BP_redPortal_C" :!type "Actor Class Reference"))
  (cast `/Game/_old/WorldObjects/BP_PortalableWall` Other
    (:`then`
      (bind _outactors (`GameplayStatics.GetAllActorsOfClass` _returnvalue))
      (if (> (`KismetArrayLibrary.Array_Length` _outactors) 0)
        (for _array_element _outactors
          (`/Engine/EditorBlueprintResources/StandardMacros.IsValid` _array_element
            (:`Is Valid`
              (`self.K2_DestroyActor` _array_element)))))
      (`|SpawnActorFromClass` _returnvalue (`KismetMathLibrary.MakeTransform` (+ HitLocation (* HitNormal 2)) (`KismetMathLibrary.Conv_VectorToRotator` HitNormal)) "AdjustIfPossibleButDontSpawnIfColliding" "OverrideRootScale" null null))
    (:`CastFailed`
      (bind _asch_zombie (cast `/Game/GameActors/Characters/AI/CH_Zombie` Other)
        (:`then`
          (`/Game/GameActors/Characters/AI/CH_Zombie.Event_Death` _asch_zombie))
        (:`CastFailed`
          _))))
  (`self.K2_DestroyActor`))

(fn `UserConstructionScript`)