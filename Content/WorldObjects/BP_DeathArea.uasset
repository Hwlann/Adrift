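; BP_DeathArea is a world trigger box that respawns players and kills zombies that overlap it.
; When a player enters, it adds ScoreValue to their score and searches all BP_Checkpoint actors for the nearest activated one.
; The player teleports to that checkpoint's location and rotation, falling back to the first PlayerStart if none is valid.
; An overlapping CH_Zombie has its EventDeath called instead.
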(event `self.Box.OnComponentBeginOverlap`
  (params (OverlappedComponent :type "PrimitiveComponent Object Reference") (OtherActor :type "Actor Object Reference") (OtherComp :type "PrimitiveComponent Object Reference") (OtherBodyIndex :type Integer) (bFromSweep :type Boolean) (SweepResult :type "HitResult Structure (by ref)"))
  (bind _nearestcheckpoint (`self.nearestCheckpoint`))
  (bind (_returnvalue_x _returnvalue_y _returnvalue_z) (`KismetMathLibrary.BreakVector` (`self.K2_GetActorLocation` _nearestcheckpoint)))
  (bind _asch_player (cast `/Game/Player/CH_player` OtherActor)
    (:`then`
      (`/Game/Player/CH_player.AddToScore` _asch_player (`self.scoreValue`))
      (set `self.currentNearestDistance` 9999999.0)
      (bind _outactors (`GameplayStatics.GetAllActorsOfClass` "/Game/WorldObjects/BP_Checkpoint.BP_Checkpoint_C"))
      (for _array_element _outactors
        (bind _returnvalue (`KismetMathLibrary.VSize` (- (`self.K2_GetActorLocation` _array_element) (`self.K2_GetActorLocation` _asch_player))))
        (if (and (< _returnvalue (`self.currentNearestDistance`)) (`/Game/WorldObjects/BP_Checkpoint.isActivate` _array_element))
          (set `self.currentNearestDistance` _returnvalue)
          (set `self.nearestCheckpoint` _array_element)))
      (`/Engine/EditorBlueprintResources/StandardMacros.IsValid` _nearestcheckpoint
        (:`Is Valid`
          (`self.K2_TeleportTo` _asch_player (`KismetMathLibrary.MakeVector` _returnvalue_x _returnvalue_y _returnvalue_z) (`self.K2_GetActorRotation` _nearestcheckpoint)))
        (:`Is Not Valid`
          (bind _outactors_2 (`GameplayStatics.GetAllActorsOfClass` "/Script/Engine.PlayerStart"))
          (bind _output (`|GetArrayItem` _outactors_2))
          (`self.K2_TeleportTo` _asch_player (`self.K2_GetActorLocation` _output) (`self.K2_GetActorRotation` _output)))))
    (:`CastFailed`
      (bind _asch_zombie (cast `/Game/Enemies/CH_Zombie` OtherActor))
      (`/Game/Enemies/CH_Zombie.Event_Death` _asch_zombie))))

(fn `UserConstructionScript`)