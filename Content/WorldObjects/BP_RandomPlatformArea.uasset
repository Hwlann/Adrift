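; BP_RandomPlatformArea is a world actor that scatters BP_ScaledPlatform actors at random positions within an area defined by its Box component.
; On BeginPlay it loops from 0 to PlatformsNbr, spawning a platform each pass with random X and Y and the box's Z.
; The range is half the unscaled extent either side of the box center, so it covers only the central part and ignores scale and rotation.
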(event `self.ReceiveBeginPlay`
  (bind _box (`self.Box`))
  (bind (_returnvalue_x _returnvalue_y _returnvalue_z) (`KismetMathLibrary.BreakVector` (`SceneComponent.K2_GetComponentLocation` _box)))
  (bind (_returnvalue_x_2 _returnvalue_y_2) (`KismetMathLibrary.BreakVector` (`BoxComponent.GetUnscaledBoxExtent` _box)))
  (bind _returnvalue (/ _returnvalue_x_2 2.0))
  (bind _returnvalue_2 (/ _returnvalue_y_2 2.0))
  (for _ (range (+ (`self.platformsNbr`) 1))
    (`|SpawnActorFromClass` "/Game/WorldObjects/BP_ScaledPlatform.BP_ScaledPlatform_C" (`KismetMathLibrary.MakeTransform` (`KismetMathLibrary.MakeVector` (`KismetMathLibrary.RandomFloatInRange` (- _returnvalue_x _returnvalue) (+ _returnvalue_x _returnvalue)) (`KismetMathLibrary.RandomFloatInRange` (- _returnvalue_y _returnvalue_2) (+ _returnvalue_y _returnvalue_2)) _returnvalue_z)) "Undefined" "OverrideRootScale" null null)))

(fn `UserConstructionScript`)