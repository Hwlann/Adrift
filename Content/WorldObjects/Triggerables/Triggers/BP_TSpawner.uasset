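; Trigger-volume spawner that creates a one-time wave of zombies and activates a linked triggerable once the wave is dead.
; When the player overlaps the box, it spawns a set number of zombies at random XY offsets around itself, with yaw taken from the player's forward vector.
; Each zombie receives a spawner reference; a death-count event fires the triggerable's Trigger when the count reaches the spawn total.
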(event `self.Box.OnComponentBeginOverlap`
  (params (OverlappedComponent :type "PrimitiveComponent Object Reference") (OtherActor :type "Actor Object Reference") (OtherComp :type "PrimitiveComponent Object Reference") (OtherBodyIndex :type Integer) (bFromSweep :type Boolean) (SweepResult :type "HitResult Structure (by ref)"))
  (bind (_returnvalue_x _returnvalue_y _returnvalue_z) (`KismetMathLibrary.BreakVector` (`self.K2_GetActorLocation` self)))
  (bind (_returnvalue_roll _returnvalue_pitch _returnvalue_yaw) (`KismetMathLibrary.BreakRotator` (`KismetMathLibrary.Conv_VectorToRotator` (* (`self.GetActorForwardVector` (`self.player`)) 180))))
  (bind _asch_player (cast `/Game/Player/CH_player` OtherActor))
  (set `self.player` _asch_player)
  (if (`self.isSpawnable`)
    (for _ (range 1 (+ (`self.spawnableZombiesCount`) 1))
      (`|SpawnActorFromClass` "/Game/Enemies/CH_Zombie.CH_Zombie_C" (`KismetMathLibrary.MakeTransform` (`KismetMathLibrary.MakeVector` (+ _returnvalue_x (`KismetMathLibrary.RandomFloatInRange` -500.0 500.0)) (+ _returnvalue_y (`KismetMathLibrary.RandomFloatInRange` -500.0 500.0)) _returnvalue_z) (`KismetMathLibrary.MakeRotator` 0.0 0.0 _returnvalue_yaw)) "AlwaysSpawn" "OverrideRootScale" null self null))
    (set `self.isSpawnable` false)))

(event `Event_AllMobsPowned`
  (`/Game/WorldObjects/Triggerables/BP_BlueprintTriggerable.Trigger` (`self.bpTriggerable`)))

(event `Event_NewMonsterDead`
  (bind _result (`/Engine/EditorBlueprintResources/StandardMacros.IncrementInt` (`self.currentDeadZombies`))
    (:`  `
      (if (== _result (`self.spawnableZombiesCount`))
        (`self.Event_AllMobsPowned`)))))

(fn `UserConstructionScript`)